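; BP_NPCPath is a spline-based NPC path actor that lays out NPC_Point actors along its Path spline at BeginPlay.
; PlacePathPoints loops from distance zero, spawning points at fixed intervals in world space until it reaches the spline length, and stores them in PathPoints.
; Before spawning, it calls SetLifeSpan with zero on existing points and clears the array, which does not itself destroy those actors.
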(event `self.ReceiveBeginPlay`
  (`self.Place Path Points`))

(event `Place Path Points`
  (set `self.Distance` 0.0)
  (for _array_element (`self.PathPoints`)
    (`/Engine/EditorBlueprintResources/StandardMacros.IsValid` _array_element
      (:`Is Valid`
        (`self.SetLifeSpan` _array_element 0.0))))
  (`KismetArrayLibrary.Array_Clear` (`self.PathPoints`))
  (bind _returnvalue (`|SpawnActorFromClass` "/Game/1_BLUEPRINTS/NavigationSystem/NPC_Point.NPC_Point_C" (`KismetMathLibrary.MakeTransform` (`SplineComponent.GetLocationAtDistanceAlongSpline` (`self.Path`) (`self.Distance`) "World")) "AlwaysSpawn" "OverrideRootScale" null null :!label _label))
  (`KismetArrayLibrary.Array_Add` (`self.PathPoints`) _returnvalue)
  (bind _output_get (set `self.Distance` (+ (`self.Distance`) 400.0)))
  (if (< _output_get (`SplineComponent.GetSplineLength` (`self.Path`)))
    (goto _label)))

(fn `UserConstructionScript`)